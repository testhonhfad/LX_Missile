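; VR-pickable missile launcher vehicle (sudb_car) that plays a staged launch sequence and can be reset.
; Fire opens Tick-driven gates in turn, separated by delays: rotate the base, rotate the shell, then move the missile, later changing its speed.
; AddSmoke attaches smoke and two-stage fire particles at the Arrow.
; Reset clears the Start flag checked after delays, closes gates, destroys particles and restores part transforms.
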(event Custom|add%20smoke
  (bind _arrow (Variables|Default|GetArrow))
  ;[1 1 1] particle system
  (bind _returnvalue (AddComponent|AddParticleSystemComponent true))
  (Utilities|Array|Add (Variables|Default|Getparticles) _returnvalue)
  (Transformation|AttachComponentToComponent _returnvalue _arrow "None" "SnapToTarget" "SnapToTarget" "KeepRelative" true)
  (bind _returnvalue_2 (AddComponent|AddParticleSystemComponent true))
  (Utilities|Array|Add (Variables|Default|Getparticles) _returnvalue_2)
  (Transformation|AttachComponentToComponent _returnvalue_2 _arrow "None" "SnapToTarget" "SnapToTarget" "KeepRelative" true)
  (Transformation|SetRelativeScale3D _returnvalue_2 "5.000000,5.000000,5.000000")
  (Transformation|SetRelativeRotation _returnvalue_2 "-90.000000, 0,0.000000" false false)
  (bind _returnvalue_3 (AddComponent|AddParticleSystemComponent true))
  (Variables|Default|Setfire1 _returnvalue_3)
  (Transformation|AttachComponentToComponent _returnvalue_3 (Variables|Default|GetArrow) "None" "SnapToTarget" "SnapToTarget" "KeepRelative" true)
  (Utilities|FlowControl|Sequence
    (:then_0
      (Utilities|FlowControl|Delay (Variables|Default|Getfiredelay))
      (if (Variables|Default|GetStart?)
        (Effects|Particles|Trails|EndTrails _returnvalue_3)
        (bind _returnvalue_4 (AddComponent|AddParticleSystemComponent true))
        (Variables|Default|Setfire2 _returnvalue_4)
        (Transformation|AttachComponentToComponent _returnvalue_4 (Variables|Default|GetArrow) "None" "SnapToTarget" "SnapToTarget" "KeepRelative" true)
        (Transformation|SetRelativeScale3D _returnvalue_4 "3.000000,3.000000,3.000000")))))

(event Custom|fire
  (bind _sudb_base (Variables|Default|Getsudb_base))
  ;[1 1 1] start system
  (Variables|Default|SetStart? true)
  ;[1 1 1] Base
  (Utilities|FlowControl|Gate true) ; enters at Open
)

(event Custom|Reset
  (bind _sudb_base (Variables|Default|Getsudb_base))
  (bind _fire1 (Variables|Default|Getfire1))
  (bind _fire2 (Variables|Default|Getfire2))
  ;[1 1 1] Reset system
  (Utilities|FlowControl|Sequence
    (:then_0
      (Variables|Default|SetStart? false))
    (:then_1
      ;[1 1 1] Base
      (Utilities|FlowControl|Gate true) ; enters at Close
    )
    (:then_2
      ;[1 1 1] Shell
      (Utilities|FlowControl|Gate true) ; enters at Close
    )
    (:then_3
      ;[1 1 1] Missle
      (Utilities|FlowControl|Gate true) ; enters at Close
    )
    (:then_4
      (Components|DestroyComponent (Variables|Default|Getparticles))
      (Utilities|IsValid _fire1
        (:Is%20Valid
          (Components|DestroyComponent _fire1))
        (:Is%20Not%20Valid
          _))
      (Utilities|IsValid _fire2
        (:Is%20Valid
          (Components|DestroyComponent _fire2))))
    (:then_5
      (Transformation|SetRelativeRotation (Variables|Default|Getsudb_base) "0, 0,-90.000000" false false)
      (Transformation|SetRelativeRotation (Variables|Default|Getsudb_shell) "0, 0,0.000000" false false)
      (Transformation|SetRelativeLocation (Variables|Default|Getsudb_missile) "0, 0, 0" false false))
    (:then_6
      (Utilities|FlowControl|DoOnce false) ; enters at Reset
    )))

(event EventTick
  (params (DeltaSeconds :type Float%20%28single-precision%29))
  (bind _sudb_base (Variables|Default|Getsudb_base))
  (Utilities|FlowControl|Sequence
    (:then_0
      ;[1 1 1] Base
      (Utilities|FlowControl|Gate true
        (:Exit
          (if (< (.roll (Variables|/Script/Engine.SceneComponent|GetRelativeRotation _sudb_base)) 0.0)
            (Transformation|AddRelativeRotation _sudb_base (Math|Rotator|MakeRotator (Variables|Default|Getshell%20speed) 0.0 0.0) false false)
            (else
              (Utilities|FlowControl|Delay (Variables|Default|Getbase%20delay))
              (if (Variables|Default|GetStart?)
                (goto _label Open)))))))
    (:then_1
      ;[1 1 1] Shell
      (Utilities|FlowControl|Gate true :!label _label
        (:Exit
          (if (> (.roll (Variables|/Script/Engine.SceneComponent|GetRelativeRotation (Variables|Default|Getsudb_shell))) -9e+01)
            (Transformation|AddRelativeRotation (Variables|Default|Getsudb_shell) (Math|Rotator|MakeRotator (* (Variables|Default|Getbase%20speed) -1.0) 0.0 0.0) false false)
            (else
              (Utilities|FlowControl|Delay (Variables|Default|Getsmokedelay))
              (if (Variables|Default|GetStart?)
                (Utilities|FlowControl|DoOnce false
                  (:Completed
                    ;[1 1 1] Add smoke
                    (CallFunction|AddSmoke)
                    (Utilities|FlowControl|Delay (Variables|Default|Getmissile%20delay))
                    (if (Variables|Default|GetStart?)
                      (Effects|Particles|Trails|EndTrails (Variables|Default|Getparticles))
                      ;[1 1 1] Second speed
                      (Utilities|FlowControl|Sequence
                        (:then_0
                          (goto _label_2 Open))
                        (:then_1
                          (Utilities|FlowControl|Delay (Variables|Default|Getspeeddelay))
                          (if (Variables|Default|GetStart?)
                            (Variables|Default|Setmissile%20speed 4e+02)))))))))))))
    (:then_2
      ;[1 1 1] Missle
      (Utilities|FlowControl|Gate true :!label _label_2
        (:Exit
          (if true
            (Transformation|AddLocalOffset (Variables|Default|Getsudb_missile) (Math|Vector|MakeVector 0.0 0.0 (Variables|Default|Getmissile%20speed)) false false)))))))

(event EventPickup
  (params (AttachTo :type Scene%20Component%20Object%20Reference))
  ;[1 1 1] pickup system
  (Physics|SetSimulatePhysics (Variables|Debug|GetStaticMeshComponent) false)
  (Transformation|AttachComponentToComponent (VehicleSound|GetRootComponent) AttachTo "None" "KeepWorld" "KeepWorld" "KeepWorld" false))

(event EventDrop
  ;[1 1 1] pickup system
  (Physics|SetSimulatePhysics (Variables|Debug|GetStaticMeshComponent) false)
  (Transformation|DetachFromActor "KeepWorld" "KeepWorld" "KeepWorld"))

(fn ConstructionScript)